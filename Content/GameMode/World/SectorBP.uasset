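; SectorBP is a world-map sector in a day-based kingdom strategy game, holding buildings, resources, population, garrison and tribute.
; On BeginPlay it registers with WorldGameMode, selects its building set, labels its tooltip, styles its spline border and forwards new-day events to population and inquisition components.
; Building increments per-type counts and unhides slot actors.
; Weekday logic drives main-UI buttons and tribute, while infection and revolution show as tooltip icons.
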(event Custom|NewDayForSector
  (Utilities|FlowControl|Sequence
    (:then_0
      (Default|NewDayforPopulationCallback (Variables|Default|GetPopulationComponent)))
    (:then_1
      (Default|NewDayforInquisitionCallback (Variables|Default|GetInquisitionComponent)))))

(event EventBeginPlay
  (Utilities|FlowControl|Sequence
    (:then_0
      (bind _asworld_game_mode (Utilities|Casting|CastToWorldGameMode (Game|GetGameMode)))
      (Default|RegisterSector _asworld_game_mode self)
      (switch Utilities|FlowControl|Switch|SwitchonBuildingsCombinations (Variables|Default|GetPossibleBuildingsClass_0)
        (:NewEnumerator3
          (Variables|Default|SetPossibleBuildings 0))
        (:NewEnumerator0
          (bind _returnvalue (AddComponent|AddCapitalBuildings))
          (Variables|Default|SetPossibleBuildings _returnvalue))
        (:NewEnumerator2
          (bind _returnvalue_2 (AddComponent|AddVillageBuildings))
          (Variables|Default|SetPossibleBuildings _returnvalue_2))))
    (:then_1
      (CallFunction|SetName))
    (:then_2
      (CallFunction|InitBorder))
    (:then_3
      (bind _asworld_game_mode_2 (Utilities|Casting|CastToWorldGameMode (Game|GetGameMode)))
      (EventDispatchers|BindEventtoNextDayDispatcher _asworld_game_mode_2 (delegate Custom|NewDayForSector)))))

(event Collision|EventActorBeginOverlap
  (params (OtherActor :type Actor%20Object%20Reference)))

(event EventTick
  (params (DeltaSeconds :type Float%20%28single-precision%29)))

(fn ConstructionScript
  (Utilities|FlowControl|Sequence
    (:then_0
      (Transformation|AttachActorToActor (Variables|Default|GetHitSphere_0) self "None" "KeepWorld" "KeepRelative" "KeepRelative" true)
      (for _array_element (Actor|GetAttachedActors self)
        (Development|PrintString (Utilities|GetDisplayName _array_element) true true "(R=1.000000,G=0.848706,B=0.000000,A=1.000000)")
        (CallFunction|InitBorder)))))

(fn SetName
  (bind _loc_name (Default|GetLocalizedSectorName (.AsMy%20Game%20Instance (Utilities|Casting|CastToMyGameInstance (Game|GetGameInstance))) (Variables|Default|GetLocName)))
  (Variables|Default|SetName_0 _loc_name)
  (bind _assector_widget (Utilities|Casting|CastToSectorWidget (UserInterface|GetUserWidgetObject (Variables|Default|GetSectorTooltip_0))))
  (Rendering|Components|TextRender|SetText (Variables|/Game/HUDs/Utils/GamePlayWidgets/SectorWidget.SectorWidget_C|GetSectorName _assector_widget) (Variables|Default|GetName_0))
  (Variables|/Game/HUDs/Utils/GamePlayWidgets/SectorWidget.SectorWidget_C|SetSectorID _assector_widget (Variables|Default|GetSectorID)))

(fn DailyActions
  (bind _returnvalue (Game|GetGameMode))
  (bind _asworld_game_mode (Utilities|Casting|CastToWorldGameMode _returnvalue))
  (switch Utilities|FlowControl|Switch|SwitchonWeekDays (Variables|/Game/TopDownBP/Blueprints/WorldGameMode.WorldGameMode_C|GetCurrentDay _asworld_game_mode)
    (:NewEnumerator1
      (CallFunction|MondayAction :!label _label))
    (:NewEnumerator3
      (bind _available (Default|SectorIsAvailable (Variables|Default|GetPopulationComponent) :!label _label_2))
      (if _available
        (Default|SetupbySector (Variables|/Game/HUDs/InWorld.InWorld_C|GetSingleTributeWidget (Variables|/Game/TopDownBP/Blueprints/WorldGameMode.WorldGameMode_C|GetMainWidget _asworld_game_mode)) (Variables|/Game/TopDownBP/Blueprints/WorldController.WorldController_C|GetChoosenSectoID (.AsWorld%20Controller (Utilities|Casting|CastToWorldController (Game|GetPlayerController 0)))))))
    (:NewEnumerator4
      (goto _label))
    (:NewEnumerator5
      (Variables|Default|SetTribute 0)
      (goto _label_2))))

(fn IsPlayerTawn
  (return (and (Utilities|Enum|Equal(Enum) (Variables|Default|GetSectorType) "NewEnumerator1") (Utilities|Enum|Equal(Enum) (Variables|Default|GetKingdome) "NewEnumerator0"))))

(fn EnableBuildingOfType
  (params (BuildingType :type BuildingType%20Enum :default "NewEnumerator3") (Enable :type Boolean))
  (for _array_element (.actors (Utilities|Array|Get(acopy) (.buildings (.Value (Utilities|Map|Find (Variables|Default|GetSlots_0) BuildingType))) (- (.Value (Utilities|Map|Find (Variables|Default|GetBuildedBuildings) BuildingType)) 1)))
    (Rendering|SetActorHiddenInGame _array_element (not Enable))))

(fn BuildBuildingActors
  (params (BuildingType :type BuildingType%20Enum :default "NewEnumerator3"))
  (CallFunction|EnableBuildingOfType BuildingType true))

(fn DestroyBuilding
  (params (BuildingType :type BuildingType%20Enum :default "NewEnumerator3"))
  (CallFunction|EnableBuildingOfType BuildingType false))

(fn IsPlayerTawnorCapital
  (bind _result (CallFunction|IsPlayerTawn))
  (return (or _result (and (Utilities|Enum|Equal(Enum) (Variables|Default|GetSectorType) "NewEnumerator2") (Utilities|Enum|Equal(Enum) (Variables|Default|GetKingdome) "NewEnumerator0")))))

(fn MondayAction
  (bind _returnvalue (Game|GetGameMode))
  (bind _asworld_game_mode (Utilities|Casting|CastToWorldGameMode _returnvalue))
  (bind _asmonday_buttons (Utilities|Casting|CastToMondayButtons (Class|WidgetSwitcher|GetActiveWidget (Variables|/Game/HUDs/InWorld.InWorld_C|GetDailyButtonsSwitcher (Variables|/Game/TopDownBP/Blueprints/WorldGameMode.WorldGameMode_C|GetMainWidget _asworld_game_mode)))))
  (Utilities|FlowControl|Sequence
    (:then_0
      (bind _result (CallFunction|IsPlayerTawnorCapital))
      (Widget|SetIsEnabled (Variables|/Game/HUDs/Utils/Buttons/MondayButtons.MondayButtons_C|GetBuildInCapital _asmonday_buttons) _result))
    (:then_1
      (bind _result_2 (CallFunction|IsPlayerTawnorCapital))
      (Widget|SetIsEnabled (Variables|/Game/HUDs/Utils/Buttons/MondayButtons.MondayButtons_C|GetHireButton _asmonday_buttons) (and _result_2 (or (Variables|/Game/TopDownBP/Blueprints/WorldGameMode.WorldGameMode_C|GetHasInquisition _asworld_game_mode) (Variables|/Game/TopDownBP/Blueprints/WorldGameMode.WorldGameMode_C|GetHasGarrison _asworld_game_mode)))))))

(fn GetSimilarBuildingsCount
  (params (BuildingID :type BuildingType%20Enum :default "NewEnumerator3"))
  (for _array_element (Variables|/Game/TopDownBP/Blueprints/World/Buildings/BuildingsComponent.BuildingsComponent_C|GetBuildingCategories (Variables|Default|GetPossibleBuildings))
    (if (Utilities|Set|Contains (.buildings _array_element) BuildingID)
      (bind _result (Utilities|Set|ToArray (.buildings _array_element)))
      (for _array_element_2 _result
        (LocalVariables|SetSumCount (+ (LocalVariables|GetSumCount) (.Value (Utilities|Map|Find (Variables|Default|GetBuildedBuildings) _array_element_2)))))
      (return (LocalVariables|GetSumCount))))
  (return (.Value (Utilities|Map|Find (Variables|Default|GetBuildedBuildings) BuildingID))))

(fn BuildandProcessBuilding
  (params (BuildingID :type BuildingType%20Enum :default "NewEnumerator3"))
  (CallFunction|BuildBuilding BuildingID)
  (Default|ProcessBuilding (Variables|Default|GetPossibleBuildings) BuildingID))

(fn BuildBuilding
  (params (BuildingType :type BuildingType%20Enum :default "NewEnumerator3"))
  (bind _buildedbuildings (Variables|Default|GetBuildedBuildings))
  (bind (_value _returnvalue) (Utilities|Map|Find _buildedbuildings BuildingType))
  (Utilities|FlowControl|Sequence
    (:then_0
      (if _returnvalue
        (Utilities|Map|Add _buildedbuildings BuildingType (+ _value 1))
        (else
          (Utilities|Map|Add _buildedbuildings BuildingType 1))))
    (:then_1
      (CallFunction|BuildBuildingActors BuildingType))))

(fn AddResource
  (params (ResourceType :type ResourceType%20Enum :default "NewEnumerator0") (Value :type Integer))
  (bind _resources (Variables|Default|GetResources))
  (Utilities|Map|Add _resources ResourceType (+ (.Value (Utilities|Map|Find _resources ResourceType)) Value)))

(fn AddFeodalResource
  (params (ResourceType :type ResourceType%20Enum :default "NewEnumerator0") (Value :type Integer))
  (bind _feodalresources (Variables|Default|GetFeodalResources))
  (Utilities|Map|Add _feodalresources ResourceType (+ (.Value (Utilities|Map|Find _feodalresources ResourceType)) Value)))

(fn CalculateAvailableTribute
  (return (Math|Float|Truncate (* (* (Variables|/Game/TopDownBP/Blueprints/World/Buildings/PopulationComponent.PopulationComponent_C|GetCurrentPopulation (Variables|Default|GetPopulationComponent)) (Variables|Default|GetTributeCoeficient)) (Variables|Default|GetProductivity)))))

(fn SetInfected
  (params (Enable :type Boolean))
  (bind _assector_widget (Utilities|Casting|CastToSectorWidget (UserInterface|GetUserWidgetObject (Variables|Default|GetSectorTooltip_0))))
  (Widget|SetVisibility (Variables|/Game/HUDs/Utils/GamePlayWidgets/SectorWidget.SectorWidget_C|GetImage_51 _assector_widget) (select Enable "Visible" "Hidden"))
  (Class|Image|SetBrush (Variables|/Game/HUDs/Utils/GamePlayWidgets/SectorWidget.SectorWidget_C|GetImage_51 _assector_widget) (select Enable (Utilities|Struct|MakeSlateBrush "(X=32.000000,Y=32.000000)" "(Left=0.000000,Top=0.000000,Right=0.000000,Bottom=0.000000)" (Utilities|Struct|MakeSlateColor "(R=1.000000,G=0.151042,B=0.159486,A=1.000000)") "/Game/MobileStarterContent/Textures/Pack1/03.03" "Image" "NoTile" "NoMirror") (Utilities|Struct|MakeSlateBrush "(X=32.000000,Y=32.000000)" "(Left=0.000000,Top=0.000000,Right=0.000000,Bottom=0.000000)" (Utilities|Struct|MakeSlateColor "(R=1.000000,G=0.000000,B=1.000000,A=0.000000)") "/Game/MobileStarterContent/Textures/Pack1/03.03" "Image" "NoTile" "NoMirror"))))

(fn InitBorder
  (bind _kingdome (Variables|Default|GetKingdome))
  (bind _border_0 (Variables|Default|GetBorder_0))
  (bind _returnvalue (Utilities|Select :Index _kingdome :NewEnumerator0 "/Game/Geometry/Materials/Team0/UnselectedSector.UnselectedSector" :NewEnumerator1 "/Game/Geometry/Materials/Team1/UnselectedSector.UnselectedSector" :NewEnumerator2 "/Game/Geometry/Materials/Team0/UnselectedSector.UnselectedSector" :NewEnumerator3 0))
  (Utilities|IsValid _border_0
    (:Is%20Valid
      (Variables|/Game/Geometry/Splines/BorderSpline.BorderSpline_C|SetSelectedMaterial _border_0 _returnvalue)
      (bind _output_get (Variables|/Game/Geometry/Splines/BorderSpline.BorderSpline_C|SetUselectedMaterial _border_0 (Utilities|Select :Index (Variables|Default|GetKingdome) :NewEnumerator0 "/Game/Geometry/Materials/Team0/DisabledMaterial.DisabledMaterial" :NewEnumerator1 "/Game/Geometry/Materials/Team1/DisabledMaterial.DisabledMaterial" :NewEnumerator2 "/Game/Geometry/Materials/Team0/DisabledMaterial.DisabledMaterial" :NewEnumerator3 0)))
      (Variables|/Game/Geometry/Splines/BorderSpline.BorderSpline_C|SetPossibleMaterial _border_0 _returnvalue)
      (for _array_element (Components|GetChildrenComponents (Variables|/Game/Geometry/Splines/BorderSpline.BorderSpline_C|GetSpline _border_0) false)
        (bind _asstatic_mesh_component (Utilities|Casting|CastToStaticMeshComponent _array_element))
        (Rendering|Material|SetMaterial _asstatic_mesh_component 0 _output_get)))))

(fn SetRevolution
  (params (Enable :type Boolean))
  (bind _assector_widget (Utilities|Casting|CastToSectorWidget (UserInterface|GetUserWidgetObject (Variables|Default|GetSectorTooltip_0))))
  (Widget|SetVisibility (Variables|/Game/HUDs/Utils/GamePlayWidgets/SectorWidget.SectorWidget_C|GetImage_51 _assector_widget) (select Enable "Visible" "Hidden"))
  (Class|Image|SetBrush (Variables|/Game/HUDs/Utils/GamePlayWidgets/SectorWidget.SectorWidget_C|GetImage_51 _assector_widget) (select Enable (Utilities|Struct|MakeSlateBrush "(X=32.000000,Y=32.000000)" "(Left=0.000000,Top=0.000000,Right=0.000000,Bottom=0.000000)" "(SpecifiedColor=(R=1.000000,G=1.000000,B=1.000000,A=1.000000),ColorUseRule=UseColor_Specified)" "/Game/MobileStarterContent/Textures/Pack1/10.10" "Image" "NoTile" "NoMirror") (Utilities|Struct|MakeSlateBrush "(X=32.000000,Y=32.000000)" "(Left=0.000000,Top=0.000000,Right=0.000000,Bottom=0.000000)" (Utilities|Struct|MakeSlateColor "(R=1.000000,G=0.000000,B=1.000000,A=0.000000)") "/Game/MobileStarterContent/Textures/Pack1/03.03" "Image" "NoTile" "NoMirror"))))

(fn ApplyParameterCHange
  (params (ParametersValues :type Map%20of%20ParameterType%20Enums%20to%20Integers :default "NewEnumerator0"))
  (bind _result (CallFunction|IsPlayerTawnorCapital))
  (if _result
    (bind _keys (Utilities|Map|Keys ParametersValues))
    (for _array_element _keys
      (switch Utilities|FlowControl|Switch|SwitchonParameterType _array_element
        (:NewEnumerator0
          (Default|BuyGarrison (Variables|Default|GetGarrisonComponent) (.Value (Utilities|Map|Find ParametersValues _array_element))))))))