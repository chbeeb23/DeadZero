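; CapitalBP is the capital actor in the world game mode, granting a Monday gold bonus scaled by its population.
; On BeginPlay it runs the parent logic, then registers itself as the Capital on WorldGameMode.
; CountMondayGoldBonus multiplies the database component's bonus by current population over maximum capital population, truncates the result and passes it to the game mode's ChangeGold.
; Nothing in this graph calls that function.
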(event EventBeginPlay
  (|CallParentFunction)
  (Variables|/Game/TopDownBP/Blueprints/WorldGameMode.WorldGameMode_C|SetCapital (.AsWorld%20Game%20Mode (Utilities|Casting|CastToWorldGameMode (Game|GetGameMode))) self))

(event Collision|EventActorBeginOverlap
  (params (OtherActor :type Actor%20Object%20Reference))
  (|CallParentFunction OtherActor) ; This node is disabled and will not be called.\nDrag off pins to build functionality.
)

(event EventTick
  (params (DeltaSeconds :type Float%20%28single-precision%29))
  (|CallParentFunction DeltaSeconds) ; This node is disabled and will not be called.\nDrag off pins to build functionality.
)

(fn ConstructionScript
  (|CallParentFunction))

(fn CountMondayGoldBonus
  (bind _returnvalue (Game|GetGameMode))
  (bind _asworld_game_mode (Utilities|Casting|CastToWorldGameMode _returnvalue))
  (bind _dbcomponent (Variables|/Game/TopDownBP/Blueprints/WorldGameMode.WorldGameMode_C|GetDBComponent _asworld_game_mode))
  (Default|ChangeGold _asworld_game_mode (Math|Float|Truncate (* (Variables|/Game/TopDownBP/Blueprints/Components/DBComponent.DBComponent_C|GetMondayGoldBonus _dbcomponent) (/ (Math|Conversions|ToFloat(Integer) (Variables|/Game/TopDownBP/Blueprints/World/Buildings/PopulationComponent.PopulationComponent_C|GetCurrentPopulation (Variables|Default|GetPopulationComponent))) (Math|Conversions|ToFloat(Integer) (Variables|/Game/TopDownBP/Blueprints/Components/DBComponent.DBComponent_C|GetCapitalMaxPopulation _dbcomponent)))))))