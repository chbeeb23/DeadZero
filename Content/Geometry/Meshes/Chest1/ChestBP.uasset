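; ChestBP is a gold pickup chest that rewards the GoodBot when it overlaps the chest component.
; On overlap it adds gold directly to the Gold variable of the first top-level InGame widget, so the UI widget holds the count.
; It then destroys the chest component, spawns an explosion emitter above the actor, and after a short delay removes the emitter and itself.
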(event OnComponentBeginOverlap(Chest)
  (params (OverlappedComponent :type Primitive%20Component%20Object%20Reference) (OtherActor :type Actor%20Object%20Reference) (OtherComp :type Primitive%20Component%20Object%20Reference) (OtherBodyIndex :type Integer) (bFromSweep :type Boolean) (SweepResult :type Hit%20Result%20Structure%20%28by%20ref%29))
  (Utilities|Casting|CastToGoodBot OtherActor)
  (bind _foundwidgets (Widget|GetAllWidgetsOfClass "/Game/HUDs/InGame.InGame_C" true))
  (Variables|/Game/HUDs/InGame.InGame_C|SetGold (Utilities|Array|Get(acopy) _foundwidgets) (+ (Variables|/Game/HUDs/InGame.InGame_C|GetGold (Utilities|Array|Get(acopy) _foundwidgets)) 1e+01))
  (Components|DestroyComponent (Variables|Default|GetChest))
  (bind _returnvalue (Effects|SpawnEmitteratLocation "/Game/MobileStarterContent/Particles/P_Explosion.P_Explosion" (+ (Transformation|GetActorLocation) "0,0.000000,100.000000")))
  (Utilities|FlowControl|Delay 0.5)
  (Components|DestroyComponent _returnvalue)
  (Actor|DestroyActor))

(event EventBeginPlay)

(event Collision|EventActorBeginOverlap
  (params (OtherActor :type Actor%20Object%20Reference)))

(event EventTick
  (params (DeltaSeconds :type Float%20%28single-precision%29)))

(fn ConstructionScript)